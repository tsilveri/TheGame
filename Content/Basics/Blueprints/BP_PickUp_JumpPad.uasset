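; Jump pad pickup that launches the overlapping character along the pad's up vector.
; DoPickUp calls LaunchCharacter, overriding both XY and Z velocity, with a velocity from GetLaunchVelocity (up vector times LaunchSpeed), so rotating the actor aims the launch.
; A DrawDebugPath event feeds that same velocity into projectile path prediction to briefly draw the trajectory from the pad's location.
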(event `DrawDebugPath`
  (`GameplayStatics.Blueprint_PredictProjectilePath_ByObjectType` :`StartPos` (`self.K2_GetActorLocation`) :`LaunchVelocity` (`self.GetLaunchVelocity`) :`ProjectileRadius` 25.0 :`ObjectTypes` (`|MakeArray` "ObjectTypeQuery3" :!type "EObjectTypeQuery Enum") :`DrawDebugType` "ForDuration" :`DrawDebugTime` 5.0))

(fn `DoPickUp`
  (params (OverlappingCharacter :type "Character Object Reference"))
  (`Character.LaunchCharacter` OverlappingCharacter (`self.GetLaunchVelocity`) true true))

(fn `GetLaunchVelocity`
  (returns (ReturnValue :type "Vector Structure"))
  (return (* (`self.GetActorUpVector`) (`self.LaunchSpeed`))))

(fn `UserConstructionScript`
  (`parent.UserConstructionScript`))