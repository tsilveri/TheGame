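; BP_NavAgent is an AI agent that patrols a looping list of nav point actors.
; It starts moving on BeginPlay using SimpleMoveToLocation toward the current point.
; Overlapping that point advances the wrapping index, while any actor overlap triggers a delayed move to the current point.
; An AI perception handler checks for sensing the player pawn but takes no action yet.
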(event `self.ReceiveBeginPlay`
  (`self.NavigateToCurrentNavPoint`))

(event `self.ReceiveActorBeginOverlap`
  (params (OtherActor :type "Actor Object Reference"))
  (`|ExecutionSequence`
    (:`then_0`
      (if (== (`|GetArrayItem` (`self.MyNavPoints`) (`self.NavIndex`)) OtherActor)
        (`/Engine/EditorBlueprintResources/StandardMacros.IncrementInt` (`self.NavIndex`))))
    (:`then_1`
      (if (> (`self.NavIndex`) (`KismetArrayLibrary.Array_LastIndex` (`self.MyNavPoints`)))
        (set `self.NavIndex` 0))
      (`KismetSystemLibrary.Delay` 3.0)
      (`self.NavigateToCurrentNavPoint`))))

(event `self.AIPerception.OnTargetPerceptionUpdated`
  (params (Actor :type "Actor Object Reference") (Stimulus :type "AIStimulus Structure"))
  (if (== (`GameplayStatics.GetPlayerPawn` 0) Actor)
    (if (`.bSuccessfullySensed` (break `AIStimulus` Stimulus))
      _)))

(fn `NavigateToCurrentNavPoint`
  (`AIBlueprintHelperLibrary.SimpleMoveToLocation` (`self.GetController`) (`self.K2_GetActorLocation` (`|GetArrayItem` (`self.MyNavPoints`) (`self.NavIndex`)))))

(fn `UserConstructionScript`)